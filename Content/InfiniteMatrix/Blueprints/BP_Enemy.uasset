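; BP_Enemy is a contact hazard that costs BP_Player one HP when it overlaps the enemy's collider, then destroys itself.
; Each hit refreshes the player's HP text, and the final one marks the player dead and shows the restart display.
; On death it destroys every health pack, with the all-enemy cleanup nested inside that loop, so enemies are cleared only when a health pack exists.
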(event `self.Enemy Collider.OnComponentBeginOverlap`
  (params (OverlappedComponent :type "PrimitiveComponent Object Reference") (OtherActor :type "Actor Object Reference") (OtherComp :type "PrimitiveComponent Object Reference") (OtherBodyIndex :type Integer) (bFromSweep :type Boolean) (SweepResult :type "HitResult Structure (by ref)"))
  (bind _asbp_player (cast `/Game/InfiniteMatrix/Blueprints/BP_Player` OtherActor))
  (`self.K2_DestroyActor`)
  (bind _hp (`/Game/InfiniteMatrix/Blueprints/BP_Player.HP` _asbp_player))
  (if (> _hp 1)
    (set `/Game/InfiniteMatrix/Blueprints/BP_Player.HP` (- _hp 1) _asbp_player)
    (`/Game/InfiniteMatrix/Blueprints/BP_Player.ChangeHPText` _asbp_player)
    (else
      (set `/Game/InfiniteMatrix/Blueprints/BP_Player.HP` 0 _asbp_player)
      (`/Game/InfiniteMatrix/Blueprints/BP_Player.ChangeHPText` _asbp_player)
      (set `/Game/InfiniteMatrix/Blueprints/BP_Player.IsDead` true _asbp_player)
      (`/Game/InfiniteMatrix/Blueprints/BP_Player.DisplayRestart` _asbp_player)
      (bind _outactors (`GameplayStatics.GetAllActorsOfClass` "/Game/InfiniteMatrix/Blueprints/BP_HealthPack.BP_HealthPack_C"))
      (for _array_element _outactors
        (`self.K2_DestroyActor` _array_element)
        (bind _outactors_2 (`GameplayStatics.GetAllActorsOfClass` "BP_Enemy_C"))
        (for _array_element_2 _outactors_2
          (`self.K2_DestroyActor` _array_element_2))))))

(fn `UserConstructionScript`)