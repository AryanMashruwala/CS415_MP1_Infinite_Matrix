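; Projectile actor that flies along world X and destroys enemies it hits, scoring for the player who fired it.
; Each tick it sweeps forward at a multiple of PlayerOrigin's ForwardSpeed, so its pace follows the player's.
; On collider overlap with a BP_Enemy it spawns an explosion particle, destroys both actors, then increments PlayerOrigin's Score and refreshes the score text.
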(event `self.ReceiveTick`
  (params (DeltaSeconds :type "Float (single-precision)"))
  (bind _playerorigin (`self.PlayerOrigin`))
  (`/Engine/EditorBlueprintResources/StandardMacros.IsValid` _playerorigin
    (:`Is Valid`
      (`self.K2_AddActorWorldOffset` (`KismetMathLibrary.MakeVector` (* 3.0 (* DeltaSeconds (`/Game/InfiniteMatrix/Blueprints/BP_Player.ForwardSpeed` _playerorigin)))) true))))

(event `self.Projectile Collider.OnComponentBeginOverlap`
  (params (OverlappedComponent :type "PrimitiveComponent Object Reference") (OtherActor :type "Actor Object Reference") (OtherComp :type "PrimitiveComponent Object Reference") (OtherBodyIndex :type Integer) (bFromSweep :type Boolean) (SweepResult :type "HitResult Structure (by ref)"))
  (bind _playerorigin (`self.PlayerOrigin`))
  (bind _asbp_enemy (cast `/Game/InfiniteMatrix/Blueprints/BP_Enemy` OtherActor))
  (bind _returnvalue_location (`KismetMathLibrary.BreakTransform` (`self.GetTransform` _asbp_enemy)))
  (`GameplayStatics.SpawnEmitterAtLocation` "/Engine/Tutorial/SubEditors/TutorialAssets/TutorialParticleSystem.TutorialParticleSystem" _returnvalue_location)
  (`self.K2_DestroyActor` _asbp_enemy)
  (`self.K2_DestroyActor`)
  (`/Engine/EditorBlueprintResources/StandardMacros.IsValid` _playerorigin
    (:`Is Valid`
      (set `/Game/InfiniteMatrix/Blueprints/BP_Player.Score` (+ (`/Game/InfiniteMatrix/Blueprints/BP_Player.Score` _playerorigin) 1) _playerorigin)
      (`/Game/InfiniteMatrix/Blueprints/BP_Player.ChangeScoreText` _playerorigin))))

(fn `UserConstructionScript`)